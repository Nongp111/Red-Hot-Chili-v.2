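; BP_Pickup_Heart is a health pickup that heals the top-down character who collects it.
; It overrides the parent pickup's HandlePickup event, runs the parent logic, then calls GetHealed on the character with its HealAmount.
; All other events are disabled stubs, and the construction script only calls the parent.
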(event EventBeginPlay
  (|CallParentFunction) ; This node is disabled and will not be called.\nDrag off pins to build functionality.
)

(event Collision|EventActorBeginOverlap
  (params (OtherActor :type Actor%20Object%20Reference))
  (|CallParentFunction OtherActor) ; This node is disabled and will not be called.\nDrag off pins to build functionality.
)

(event EventTick
  (params (DeltaSeconds :type Float%20%28single-precision%29))
  (|CallParentFunction DeltaSeconds) ; This node is disabled and will not be called.\nDrag off pins to build functionality.
)

(event EventHandlePickup
  (params (Topdown :type BP%20Topdown%20Object%20Reference))
  (|CallParentFunction Topdown)
  (Default|GetHealed Topdown (Variables|Default|GetHeal%20Amount)))

(fn ConstructionScript
  (|CallParentFunction))