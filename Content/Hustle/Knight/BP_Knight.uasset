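; BP_Knight is a sprite-based knight character that damages BP_Topdown when its hurt box overlaps that actor's hurt box.
; WalkTowards moves it and flips the sprite by X direction, unless it is stunned or defeated.
; Damage reduces BPCHealth, drives timeline velocity knockback away from the damage causer, and flashes the sprite red.
; On defeat it disables the hurt box and destroys itself after a delay; the death VFX spawn is unconnected.
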(event OnComponentBeginOverlap(HurtBox)
  (params (OverlappedComponent :type Primitive%20Component%20Object%20Reference) (OtherActor :type Actor%20Object%20Reference) (OtherComp :type Primitive%20Component%20Object%20Reference) (OtherBodyIndex :type Integer) (bFromSweep :type Boolean) (SweepResult :type Hit%20Result%20Structure%20%28by%20ref%29))
  (bind _asbp_topdown (Utilities|Casting|CastToBP_Topdown OtherActor))
  (if (== (Variables|/Game/BP_Topdown.BP_Topdown_C|GetHurtBox _asbp_topdown) OtherComp)
    (Game|Damage|ApplyDamage _asbp_topdown 2.0 0 self)))

(event Custom|GetKnockedBack
  (params (Attacker :type Actor%20Object%20Reference))
  (Variables|Default|SetKnockBackDirection (Math|Vector|GetForwardVector (Math|Rotator|FindLookatRotation (Transformation|GetActorLocation Attacker) (Transformation|GetActorLocation))))
  (Components|Timeline|SetPlayRate (Variables|Default|GetKnockBackMovement) 5.0)
  (Timeline|KnockBackMovement PlayFromStart
    (:Update
      (Variables|/Script/Engine.MovementComponent|SetVelocity (Variables|Character|GetCharacterMovement) (* (Variables|Default|GetKnockBackDirection) (Variables|Default|GetKnockBackStrength))))))

(event Custom|WalkTowards
  (params (WorldDirection :type Vector))
  (bind _sprite (Variables|Default|GetSprite))
  (if (and (not (Variables|/Game/Component/BPC_Health.BPC_Health_C|GetIsDefeated (Variables|Default|GetBPC_Health))) (not (Variables|Default|GetIsStunned)))
    (Pawn|Input|AddMovementInput WorldDirection 1.0 false)
    (if (> (.X (Math|Vector|BreakVector WorldDirection)) 0.0)
      (Transformation|SetRelativeScale3D _sprite "-1.000000,1.000000,1.000000")
      (else
        (Transformation|SetRelativeScale3D _sprite "1.000000,1.000000,1.000000")))))

(event Custom|SetStun
  (Variables|Default|SetIsStunned true)
  (Utilities|FlowControl|RetriggerableDelay (Variables|Default|GetStunDuration))
  (Variables|Default|SetIsStunned false))

(event Custom|HandlDefeat
  (Collision|SetCollisionEnabled (Variables|Default|GetHurtBox) "NoCollision")
  (Utilities|FlowControl|Delay (Variables|Default|GetDespawnDuration))
  (Actor|DestroyActor))

(event Custom|FlashSprite
  (Sprite|SetSpriteColor (Variables|Default|GetSprite) "(R=1.000000,G=0.000000,B=0.000000,A=1.000000)")
  (Utilities|FlowControl|RetriggerableDelay (Variables|Default|GetFlashDuration))
  (Sprite|SetSpriteColor (Variables|Default|GetSprite) "(R=1.000000,G=1.000000,B=1.000000,A=1.000000)"))

(event EventBeginPlay
  (|CallParentFunction) ; This node is disabled and will not be called.\nDrag off pins to build functionality.
)

(event Game|Damage|EventAnyDamage
  (params (Damage :type Float%20%28single-precision%29) (DamageType :type Damage%20Type%20Object%20Reference) (InstigatedBy :type Controller%20Object%20Reference) (DamageCauser :type Actor%20Object%20Reference))
  (Default|DecreaseHealth (Variables|Default|GetBPC_Health) Damage)
  (CallFunction|GetKnockedBack DamageCauser)
  (CallFunction|FlashSprite)
  (if (Variables|/Game/Component/BPC_Health.BPC_Health_C|GetIsDefeated (Variables|Default|GetBPC_Health))
    (CallFunction|HandlDefeat)))

(event EventTick
  (params (DeltaSeconds :type Float%20%28single-precision%29))
  (|CallParentFunction DeltaSeconds) ; This node is disabled and will not be called.\nDrag off pins to build functionality.
)

(event Collision|EventActorBeginOverlap
  (params (OtherActor :type Actor%20Object%20Reference))
  (|CallParentFunction OtherActor) ; This node is disabled and will not be called.\nDrag off pins to build functionality.
)

(fn ConstructionScript
  (|CallParentFunction))