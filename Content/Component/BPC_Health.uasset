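; Health component that tracks current health, defeat state and temporary invincibility for its owning actor.
; Health starts at max on BeginPlay; decrease and increase functions clamp it between zero and max, with decrease flagging defeat at zero.
; SetInvincibility raises a flag for a set duration via a Delay, and CanBeDamged reports false while defeated or invincible, though DecreaseHealth does not check it.
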(event Custom|SetInvincibility
  (Variables|Default|SetIsInvincible true)
  (Utilities|FlowControl|Delay (Variables|Default|GetinvincibilityDuration))
  (Variables|Default|SetIsInvincible false))

(event EventBeginPlay
  (Variables|Default|SetCurrenHealth (Variables|Default|GetMaxHealth)))

(event EventTick
  (params (DeltaSeconds :type Float%20%28single-precision%29)))

(fn DecreaseHealth
  (params (IncomingDamage :type Float%20%28double-precision%29))
  (Variables|Default|SetCurrenHealth (Math|Float|Max(Float) (- (Variables|Default|GetCurrenHealth) IncomingDamage) 0.0))
  (Variables|Default|SetIsDefeated (<= (Variables|Default|GetCurrenHealth) 0.0)))

(fn CanbeDamged
  (return (and (not (Variables|Default|GetIsDefeated)) (not (Variables|Default|GetIsInvincible)))))

(fn IncreaseHealth
  (params (IncreaseAmount :type Float%20%28double-precision%29))
  (Variables|Default|SetCurrenHealth (Math|Float|Min(Float) (+ IncreaseAmount (Variables|Default|GetCurrenHealth)) (Variables|Default|GetMaxHealth))))