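; BP_Advance_Spawner is a trigger-based enemy spawner that ambushes the top-down player with knight and dog AI in two waves.
; BeginPlay caches the player pawn as BP_Topdown, and only that pawn's first overlap with the Box fires SpawnEnemy, via a DoOnce.
; SpawnEnemy spawns the first wave immediately and the second after a short Delay, placing each enemy at its own Billboard component's location and rotation.
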(event OnComponentBeginOverlap(Box)
  (params (OverlappedComponent :type Primitive%20Component%20Object%20Reference) (OtherActor :type Actor%20Object%20Reference) (OtherComp :type Primitive%20Component%20Object%20Reference) (OtherBodyIndex :type Integer) (bFromSweep :type Boolean) (SweepResult :type Hit%20Result%20Structure%20%28by%20ref%29))
  (if (== OtherActor (Variables|Default|GetAs%20BP%20Topdown))
    (Utilities|FlowControl|DoOnce false
      (:Completed
        (CallFunction|SpawnEnemy)))))

(event Custom|SpawnEnemy
  (bind _billboard3 (Variables|Default|GetBillboard3))
  (bind _billboard4 (Variables|Default|GetBillboard4))
  (bind _billboard6 (Variables|Default|GetBillboard6))
  (bind _billboard (Variables|Default|GetBillboard))
  (bind _billboard12 (Variables|Default|GetBillboard12))
  (bind _billboard11 (Variables|Default|GetBillboard11))
  (bind _billboard10 (Variables|Default|GetBillboard10))
  (Utilities|FlowControl|Sequence
    (:then_0
      (Utilities|FlowControl|Sequence
        (:then_0
          (AI|SpawnAIFromClass "/Game/Hustle/Knight/BP_Knight.BP_Knight_C" 0 (Transformation|GetWorldLocation _billboard) (Transformation|GetWorldRotation _billboard) false 0))
        (:then_2
          (AI|SpawnAIFromClass "/Game/Hustle/Dog/BP_Dog.BP_Dog_C" 0 (Transformation|GetWorldLocation _billboard3) (Transformation|GetWorldRotation _billboard3) false 0))
        (:then_4
          (AI|SpawnAIFromClass "/Game/Hustle/Dog/BP_Dog.BP_Dog_C" 0 (Transformation|GetWorldLocation _billboard6) (Transformation|GetWorldRotation _billboard6) false 0))
        (:then_5
          (AI|SpawnAIFromClass "/Game/Hustle/Dog/BP_Dog.BP_Dog_C" 0 (Transformation|GetWorldLocation _billboard4) (Transformation|GetWorldRotation _billboard4) false 0))))
    (:then_1
      (Utilities|FlowControl|Delay 5.0)
      (Utilities|FlowControl|Sequence
        (:then_0
          (AI|SpawnAIFromClass "/Game/Hustle/Knight/BP_Knight.BP_Knight_C" 0 (Transformation|GetWorldLocation _billboard12) (Transformation|GetWorldRotation _billboard12) false 0))
        (:then_1
          (AI|SpawnAIFromClass "/Game/Hustle/Knight/BP_Knight.BP_Knight_C" 0 (Transformation|GetWorldLocation _billboard11) (Transformation|GetWorldRotation _billboard11) false 0))
        (:then_2
          (AI|SpawnAIFromClass "/Game/Hustle/Dog/BP_Dog.BP_Dog_C" 0 (Transformation|GetWorldLocation _billboard10) (Transformation|GetWorldRotation _billboard10) false 0))))))

(event EventBeginPlay
  (bind _asbp_topdown (Utilities|Casting|CastToBP_Topdown (Game|Player|GetPlayerPawn 0)))
  (Variables|Default|SetAs%20BP%20Topdown _asbp_topdown))

(fn ConstructionScript)