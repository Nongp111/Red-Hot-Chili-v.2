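; Breakable jar actor that drops a heart pickup when it takes damage.
; Any damage starts a short delay, then DropItem spawns an enlarged BP_Pickup_Heart at the Billboard's transform, a glass-break sound plays and the jar is destroyed.
; A HurtBox overlap with BP_Topdown's own HurtBox calls ApplyDamage with the jar as causer, but no damaged actor is set on that call.
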(event OnComponentBeginOverlap(HurtBox)
  (params (OverlappedComponent :type Primitive%20Component%20Object%20Reference) (OtherActor :type Actor%20Object%20Reference) (OtherComp :type Primitive%20Component%20Object%20Reference) (OtherBodyIndex :type Integer) (bFromSweep :type Boolean) (SweepResult :type Hit%20Result%20Structure%20%28by%20ref%29))
  (bind _asbp_topdown (Utilities|Casting|CastToBP_Topdown OtherActor))
  (if (== (Variables|/Game/BP_Topdown.BP_Topdown_C|GetHurtBox _asbp_topdown) OtherComp)
    (Game|Damage|ApplyDamage 0 1.0 0 self)))

(event Custom|DropItem
  (bind _billboard (Variables|Default|GetBillboard))
  (Game|SpawnActorfromClass "/Game/Pickups/BP_Pickup_Heart.BP_Pickup_Heart_C" (Math|Transform|MakeTransform (Transformation|GetWorldLocation _billboard) (Transformation|GetWorldRotation _billboard) "1.500000,1.500000,1.500000") "Undefined" "MultiplyWithRoot" 0 0))

(event EventBeginPlay)

(event Collision|EventActorBeginOverlap
  (params (OtherActor :type Actor%20Object%20Reference)))

(event EventTick
  (params (DeltaSeconds :type Float%20%28single-precision%29)))

(event Game|Damage|EventAnyDamage
  (params (Damage :type Float%20%28single-precision%29) (DamageType :type Damage%20Type%20Object%20Reference) (InstigatedBy :type Controller%20Object%20Reference) (DamageCauser :type Actor%20Object%20Reference))
  (Utilities|FlowControl|Delay 0.3)
  (CallFunction|DropItem)
  (Audio|PlaySound2D "/Game/Sounds/glass-break-2-80964.glass-break-2-80964" 1.0 1.0 0.0 0 0)
  (Actor|DestroyActor))

(fn ConstructionScript)